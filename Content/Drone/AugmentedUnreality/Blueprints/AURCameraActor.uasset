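; Augmented reality camera actor that mirrors a tracking driver's pose and displays its feed on a Screen component.
; On BeginPlay it constructs and initializes the driver from DriverClass, hands it to the Screen, and applies a default FOV.
; Each Tick it moves the actor to the driver's newly available orientation transform.
; Driver parameter changes update camera FOV and screen size together; EndPlay shuts both down.
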(event `self.ReceiveBeginPlay`
  (bind _driverinstance (`self.DriverInstance`))
  ;[1 1 1] Initialize (create driver) if not initialized earlier
  (`/Engine/EditorBlueprintResources/StandardMacros.IsValid` _driverinstance
    (:`Is Not Valid`
      (`self.Initialize`)
      (add `AURDriver.OnCameraParametersChange` _driverinstance (delegate `CameraParametersChanged`)))))

(event `CameraParametersChanged`
  (params (Driver :type "AURDriver Object Reference"))
  (`self.SetFOV` (`KismetMathLibrary.BreakVector2D` (`AURDriver.GetFieldOfView` (`self.DriverInstance`)))))

(event `self.ReceiveEndPlay`
  (params (EndPlayReason :type "EEndPlayReason Enum" :default "Destroyed"))
  (`ActorComponent.Deactivate` (`self.Screen`))
  (`AURDriver.Shutdown` (`self.DriverInstance`)))

(event `self.ReceiveTick`
  (params (DeltaSeconds :type "Float (single-precision)"))
  (bind _driverinstance (`self.DriverInstance`))
  (if (`AURDriver.IsNewOrientationAvailable` _driverinstance)
    (bind _returnvalue (`AURDriver.GetOrientation` _driverinstance))
    (`self.K2_SetActorTransform` _returnvalue)))

(fn `Initialize`
  (bind _returnvalue (`|GenericCreateObject` (`self.DriverClass`) self))
  (bind _output_get (set `self.DriverInstance` _returnvalue))
  (`AURDriver.Initialize` _output_get)
  (`AURVideoScreenBase.Initialize` (`self.Screen`) _output_get)
  (`self.SetFOV` (`self.DefaultFOV`)))

(fn `SetFOV`
  (params (FOV :type "Float (double-precision)"))
  (if (!= FOV (`self.CurrentFOV`))
    (bind _output_get (set `self.CurrentFOV` FOV))
    (`CameraComponent.SetFieldOfView` (`self.CameraComponent`) _output_get)
    (`AURVideoScreenBase.SetSizeForFOV` (`self.Screen`) _output_get)))

(fn `UserConstructionScript`)